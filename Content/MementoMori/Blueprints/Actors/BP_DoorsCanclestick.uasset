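; Interactable hinged door that opens and closes with audio and a timeline meant to lerp hinge yaw, with lock and auto-close options.
; On interact it asks BP_CrossManager to check the crosses; a failed check spawns a Baphomet that plays a jumpscare after a short delay, while the door logic still runs.
; Open time sets the timeline's play rate, and interaction is disabled once used until the timeline's finish handler restores it.
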(event Custom|CloseDoor
  (Variables|Default|SetIsOpen false)
  (Components|Timeline|ReversefromEnd (Variables|Default|GetTimeLine_Open))
  (if (< (Variables|Default|GetOpenTime) 1.0) ; xD
    _
    (else
      (Audio|Components|Audio|Play (Variables|Default|GetCloseAudio) 0.0)))
  (Development|PrintString "close"))

(event EventBeginInteract
  (params (Caller :type Actor%20Object%20Reference))
  (bind _returnvalue (Actor|GetActorOfClass "/Game/MementoMori/Blueprints/Actors/BP_CrossManager.BP_CrossManager_C"))
  (if (Default|CheckCrosses _returnvalue)
    (Variables|Default|SetShouldInteract false :!label _label)
    (if (Variables|Default|GetIsLocked)
      (Development|PrintString "locked")
      (elif (Variables|Default|GetIsOpen)
        (Variables|Default|SetIsOpen false)
        (CallFunction|CloseDoor)
        (else
          (Development|PrintString "unlocked")
          (Variables|Default|SetIsOpen true)
          (Variables|Default|SetTargetYaw (* (Variables|Default|GetOpenAngle) (Variables|Default|GetHingeSideSign)))
          (Components|Timeline|PlayfromStart (Variables|Default|GetTimeLine_Open))
          (Audio|Components|Audio|Play (Variables|Default|GetOpenAudio) 0.0))))
    (else
      (Utilities|FlowControl|Sequence
        (:then_0
          (bind _returnvalue_2 (Game|SpawnActorfromClass "/Game/MementoMori/Blueprints/Character/BP_MementoMoriBaphomet.BP_MementoMoriBaphomet_C" (Transformation|GetWorldTransform (Variables|Default|GetScene)) "Undefined" "MultiplyWithRoot" 0 0))
          (Utilities|FlowControl|Delay 1.0)
          (Default|Jumpscare1 _returnvalue_2 "/Game/MementoMori/Character/AM_Jumpscare2.AM_Jumpscare2"))
        (:then_1
          (goto _label))))))

(event EventBeginPlay
  (bind _opentime (Variables|Default|GetOpenTime))
  (Variables|Default|SetClosedYaw (.Yaw (Math|Rotator|BreakRotator (Variables|/Script/Engine.SceneComponent|GetRelativeRotation (Variables|Default|GetHinge)))))
  (CallFunction|SetOpenTime _opentime)
  (Variables|Default|SetInitialOpenTime _opentime))

(fn ConstructionScript)

(fn SetOpenTime
  (params (OpenTimeToSet :type Float%20%28double-precision%29))
  (bind _output_get (Variables|Default|SetOpenTime OpenTimeToSet))
  (Components|Timeline|SetPlayRate (Variables|Default|GetTimeLine_Open) (/ 1.0 _output_get)))

(fn CanInteract
  (params (Caller :type Actor%20Object%20Reference))
  (return (Variables|Default|GetShouldInteract)))

(fn GetInteractionMessage
  (params (Caller :type Actor%20Object%20Reference))
  (return ""))

(fn IsOngoingInteraction
  (return false))