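; BP_Cross is an interactable cross actor that toggles between its placed rotation and a target rotation.
; Each interaction plays or reverses a timeline that lerps the actor's rotation, blocking further interaction until it finishes.
; The construction script captures the initial rotation, and BeginPlay snaps the cross to the target rotation if it starts flagged as rotated.
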(event EventBeginPlay
  (if (Variables|Default|GetRotated)
    (Transformation|SetActorRotation (Variables|Default|GetRotatedRotation))))

(event EventBeginInteract
  (params (Caller :type Actor%20Object%20Reference))
  (bind _rotatecrosstimeline (Variables|Default|GetRotateCrossTimeline))
  (Variables|Default|SetCanCrossInteract false)
  (if (Variables|Default|GetRotated)
    (Components|Timeline|ReversefromEnd _rotatecrosstimeline)
    (Variables|Default|SetRotated false)
    (else
      (Components|Timeline|PlayfromStart _rotatecrosstimeline)
      (Variables|Default|SetRotated true))))

(fn ConstructionScript
  (Variables|Default|SetInitialRotation (Transformation|GetActorRotation)))

(fn CanInteract
  (params (Caller :type Actor%20Object%20Reference))
  (return (Variables|Default|GetCanCrossInteract)))

(fn GetInteractionMessage
  (params (Caller :type Actor%20Object%20Reference))
  (return ""))

(fn IsOngoingInteraction
  (return false))