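; Pentagram trigger actor that summons the Baphomet enemy when a candlestick enters its box.
; On the first such overlap it spawns BP_MementoMoriBaphomet at the referenced EvilSpawnPoint's transform, with a flag blocking repeat spawns.
; It then hands the spawned Baphomet to the candlestick's Evil reference and turns off the player hero's panic mode.
; Overlaps also print leftover debug strings.
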(event OnComponentBeginOverlap(Box)
  (params (OverlappedComponent :type Primitive%20Component%20Object%20Reference) (OtherActor :type Actor%20Object%20Reference) (OtherComp :type Primitive%20Component%20Object%20Reference) (OtherBodyIndex :type Integer) (bFromSweep :type Boolean) (SweepResult :type Hit%20Result%20Structure%20%28by%20ref%29))
  (bind _asbp_candlestick (Utilities|Casting|CastToBP_Candlestick OtherActor)
    (:then
      (Development|PrintString "yeaaaa")
      (if (not (Variables|Default|GetAlreadySpawned))
        (bind _returnvalue (Game|SpawnActorfromClass "/Game/MementoMori/Blueprints/Character/BP_MementoMoriBaphomet.BP_MementoMoriBaphomet_C" (Transformation|GetWorldTransform (Variables|/Game/MementoMori/Blueprints/Actors/BP_EvilSpawn.BP_EvilSpawn_C|GetSpawnPoint (Variables|Default|GetEvilSpawnPoint))) "Undefined" "MultiplyWithRoot" 0 0))
        (Variables|Default|SetAlreadySpawned true)
        (Variables|/Game/MementoMori/Blueprints/Actors/BP_Candlestick.BP_Candlestick_C|SetEvil _asbp_candlestick _returnvalue)
        (bind _asbp_memento_mori_hero (Utilities|Casting|CastToBP_MementoMoriHero (Game|Player|GetPlayerPawn 0)))
        (Variables|/Game/MementoMori/Blueprints/Character/BP_MementoMoriHero.BP_MementoMoriHero_C|SetIsPanicMode _asbp_memento_mori_hero false)))
    (:CastFailed
      (Development|PrintString "naaaah"))))

(event EventBeginPlay)

(event Collision|EventActorBeginOverlap
  (params (OtherActor :type Actor%20Object%20Reference)))

(event EventTick
  (params (DeltaSeconds :type Float%20%28single-precision%29)))

(fn ConstructionScript)