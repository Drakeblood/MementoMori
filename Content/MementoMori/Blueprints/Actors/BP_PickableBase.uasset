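; BP_PickableBase is a base actor for items the player can interact with to pick up and hold.
; BeginInteract marks the item picked and passes a component, location and rotation from three getter functions to the caller's AC_PickUp component, and EndInteract releases it.
; The getters return empty or zero defaults, apparently for child Blueprints to override.
; Interaction is always allowed, reported as ongoing, and shows no message.
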(event EventBeginPlay)

(event Collision|EventActorBeginOverlap
  (params (OtherActor :type Actor%20Object%20Reference)))

(event EventTick
  (params (DeltaSeconds :type Float%20%28single-precision%29)))

(event EventBeginInteract
  (params (Caller :type Actor%20Object%20Reference))
  (if (not (Variables|Default|GetIsPicked))
    (Variables|Default|SetIsPicked true)
    (Default|PickUpItem (Actor|GetComponentbyClass Caller "/Game/MementoMori/Blueprints/Components/AC_PickUp.AC_PickUp_C") (CallFunction|GetComponentforPickUp) "None" (CallFunction|GetLocationforPickUp) (CallFunction|GetRotationforPickUp))))

(event EventEndInteract
  (params (Caller :type Actor%20Object%20Reference))
  (Variables|Default|SetIsPicked false)
  (Default|ReleaseItem (Actor|GetComponentbyClass Caller "/Game/MementoMori/Blueprints/Components/AC_PickUp.AC_PickUp_C")))

(fn ConstructionScript)

(fn GetComponentforPickUp
  (return 0))

(fn GetLocationforPickUp
  (return "0, 0, 0"))

(fn GetRotationforPickUp
  (return "0, 0, 0"))

(fn CanInteract
  (params (Caller :type Actor%20Object%20Reference))
  (return true))

(fn GetInteractionMessage
  (params (Caller :type Actor%20Object%20Reference))
  (return ""))

(fn IsOngoingInteraction
  (return true))