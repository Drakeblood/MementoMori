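; Candlestick puzzle actor that decides the fight against Baphomet by tracking lit child candles through fired up/down events.
; Lighting an even-ID candle extinguishes the lit set and speeds up Baphomet; three odd ones start the final phase and Baphomet's trail.
; Tick then waits for one to go out: any remaining multiple of three resets and speeds him up, otherwise he is destroyed and the hero's panic ends.
; Also exposes its mesh for pickup.
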(event Custom|CheckIfAllLightenUp
  (if (== (Utilities|Array|Length (Variables|Default|GetFiredUpCandles)) 3)
    (if (CallFunction|AllItemsAreOdd)
      (Development|PrintString "done")
      (Variables|Default|SetIsFinalFaze true)
      (bind _asbp_memento_mori_baphomet (Utilities|Casting|CastToBP_MementoMoriBaphomet (Variables|Default|GetEvil)))
      (Variables|/Game/MementoMori/Blueprints/Character/BP_MementoMoriBaphomet.BP_MementoMoriBaphomet_C|SetShouldSpawnTrail _asbp_memento_mori_baphomet true)
      (else
        (for _array_element (Variables|Default|GetFiredUpCandles)
          (Default|Extinguish _array_element))))
    (else
      (Development|PrintString "not yet"))))

(event Custom|CandleFiredUp
  (params (CandleRef :type BP%20Candle%20Object%20Reference))
  (Utilities|Array|Add (Variables|Default|GetFiredUpCandles) CandleRef)
  (if (== (Math|Integer|%(Integer) (Variables|/Game/MementoMori/Blueprints/Actors/BP_Candle.BP_Candle_C|GetID CandleRef) 2) 0)
    (Development|PrintString "failed")
    (for _array_element (Variables|Default|GetFiredUpCandles)
      (Default|Extinguish _array_element))
    (bind _asbp_memento_mori_baphomet (Utilities|Casting|CastToBP_MementoMoriBaphomet (Variables|Default|GetEvil)))
    (Variables|/Script/Engine.CharacterMovementComponent|SetMaxWalkSpeed (Variables|/Script/Engine.Character|GetCharacterMovement _asbp_memento_mori_baphomet) (+ (Variables|/Script/Engine.CharacterMovementComponent|GetMaxWalkSpeed (Variables|/Script/Engine.Character|GetCharacterMovement _asbp_memento_mori_baphomet)) 1e+02))
    (else
      (Development|PrintString "still fine")
      (CallFunction|CheckifAllLightenUp))))

(event Custom|CandleFiredDown
  (params (CandleRef :type BP%20Candle%20Object%20Reference))
  (Utilities|Array|RemoveItem (Variables|Default|GetFiredUpCandles) CandleRef))

(event EventBeginPlay
  (for _array_element (Components|GetChildrenComponents (Variables|Default|GetCandles) false)
    (EventDispatchers|BindEventtoFiredUp (.AsBP%20Candle (Utilities|Casting|CastToBP_Candle (Variables|/Script/Engine.ChildActorComponent|GetChildActor (.AsChild%20Actor%20Component (Utilities|Casting|CastToChildActorComponent _array_element))))) (delegate Custom|CandleFiredUp))
    (EventDispatchers|BindEventtoFiredDown (.AsBP%20Candle (Utilities|Casting|CastToBP_Candle (Variables|/Script/Engine.ChildActorComponent|GetChildActor (.AsChild%20Actor%20Component (Utilities|Casting|CastToChildActorComponent _array_element))))) (delegate Custom|CandleFiredDown))))

(event EventTick
  (params (DeltaSeconds :type Float%20%28single-precision%29))
  (bind _firedupcandles (Variables|Default|GetFiredUpCandles))
  (if (Variables|Default|GetIsFinalFaze)
    (Variables|Default|SetIsCorrect true)
    (if (< (Utilities|Array|Length _firedupcandles) 3)
      (for _array_element _firedupcandles
        (if (== (Math|Integer|%(Integer) (Variables|/Game/MementoMori/Blueprints/Actors/BP_Candle.BP_Candle_C|GetID _array_element) 3) 0)
          (Variables|Default|SetIsCorrect false)))
      (if (Variables|Default|GetIsCorrect)
        (Development|PrintString "correct")
        (Variables|Default|SetIsFinalFaze false)
        (Actor|DestroyActor (Variables|Default|GetEvil))
        (Development|PrintString "Player wins!")
        (bind _asbp_memento_mori_hero (Utilities|Casting|CastToBP_MementoMoriHero (Game|Player|GetPlayerPawn 0)))
        (Variables|/Game/MementoMori/Blueprints/Character/BP_MementoMoriHero.BP_MementoMoriHero_C|SetIsPanicMode _asbp_memento_mori_hero false)
        (else
          (Development|PrintString "failed")
          (for _array_element_2 (Variables|Default|GetFiredUpCandles)
            (Default|Extinguish _array_element_2))
          (Variables|Default|SetIsFinalFaze false)
          (bind _asbp_memento_mori_baphomet (Utilities|Casting|CastToBP_MementoMoriBaphomet (Variables|Default|GetEvil)))
          (Variables|/Script/Engine.CharacterMovementComponent|SetMaxWalkSpeed (Variables|/Script/Engine.Character|GetCharacterMovement _asbp_memento_mori_baphomet) (+ (Variables|/Script/Engine.CharacterMovementComponent|GetMaxWalkSpeed (Variables|/Script/Engine.Character|GetCharacterMovement _asbp_memento_mori_baphomet)) 1e+02)))))))

(fn ConstructionScript
  (|CallParentFunction))

(fn GetComponentforPickUp
  (return (Variables|Default|GetStaticMesh)))

(fn GetLocationforPickUp
  (return (Transformation|GetWorldLocation (Variables|Default|GetStaticMesh))))

(fn GetRotationforPickUp
  (return (Transformation|GetWorldRotation (Variables|Default|GetStaticMesh))))

(fn AllItemsAreOdd
  (Variables|Default|SetIsOdd true)
  (for _array_element (Variables|Default|GetFiredUpCandles)
    (if (== (Math|Integer|%(Integer) (Variables|/Game/MementoMori/Blueprints/Actors/BP_Candle.BP_Candle_C|GetID _array_element) 2) 0)
      (Variables|Default|SetIsOdd false)))
  (return (Variables|Default|GetIsOdd)))