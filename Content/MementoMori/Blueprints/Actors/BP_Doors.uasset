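; BP_Doors is an interactable hinged door that can be locked and toggles open or closed on interaction.
; BeginPlay caches the closed yaw and scales the timeline play rate by OpenTime.
; Interaction plays or reverses the timeline, whose update lerps the Hinge yaw toward a target set by open angle and hinge side.
; The timeline's finish handler calls DoorOpened and optionally schedules an auto-close timer.
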(event Custom|CloseDoor
  (Variables|Default|SetIsOpen false)
  (Components|Timeline|ReversefromEnd (Variables|Default|GetTimeLine_Open))
  (Development|PrintString "close"))

(event EventBeginInteract
  (params (Caller :type Actor%20Object%20Reference))
  (if (Variables|Default|GetIsLocked)
    (Development|PrintString "locked")
    (elif (Variables|Default|GetIsOpen)
      (Variables|Default|SetIsOpen false)
      (CallFunction|CloseDoor)
      (else
        (Development|PrintString "unlocked")
        (Variables|Default|SetIsOpen true)
        (Variables|Default|SetTargetYaw (* (Variables|Default|GetOpenAngle) (Variables|Default|GetHingeSideSign)))
        (Components|Timeline|PlayfromStart (Variables|Default|GetTimeLine_Open))))))

(event EventBeginPlay
  (Variables|Default|SetClosedYaw (.Yaw (Math|Rotator|BreakRotator (Variables|/Script/Engine.SceneComponent|GetRelativeRotation (Variables|Default|GetHinge)))))
  (Components|Timeline|SetPlayRate (Variables|Default|GetTimeLine_Open) (/ 1.0 (Variables|Default|GetOpenTime))))

(fn ConstructionScript)

(fn CanInteract
  (params (Caller :type Actor%20Object%20Reference))
  (return true))

(fn GetInteractionMessage
  (params (Caller :type Actor%20Object%20Reference))
  (return ""))

(fn IsOngoingInteraction
  (return false))