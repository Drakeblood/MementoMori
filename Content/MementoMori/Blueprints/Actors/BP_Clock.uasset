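; BP_Clock is a clock actor that animates a short and a long pointer, starting on BeginPlay.
; ConfigClock counts the cycle, captures pointer rotations, offsets the short pointer's target by a per-cycle step and plays TimelineClock.
; The timeline's update logic lerps both pointers, and its finish logic repeats ConfigClock and plays ClockSound while the cycle count is below five.
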(event Custom|ConfigClock
  (Math|Integer|IncrementInt (Variables|Default|GetClockCycles)
    (:%20%20
      (bind _output_get (Variables|Default|SetRotatorShortStart (Transformation|GetWorldRotation (Variables|Default|GetPointerShort))))
      (Variables|Default|SetRotatorShort (Math|Rotator|CombineRotators _output_get (Variables|Default|GetRotatorShortMovePerCycle)))
      (Variables|Default|SetRotatorLongStart (Transformation|GetWorldRotation (Variables|Default|GetPointerLong)))
      (Components|Timeline|PlayfromStart (Variables|Default|GetTimeline%20Clock))
      (Development|PrintString "clock play"))))

(event EventBeginPlay
  (CallFunction|ConfigClock))

(event Collision|EventActorBeginOverlap
  (params (OtherActor :type Actor%20Object%20Reference)))

(event EventTick
  (params (DeltaSeconds :type Float%20%28single-precision%29)))

(fn ConstructionScript)