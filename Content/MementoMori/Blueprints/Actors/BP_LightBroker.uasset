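; BP_LightBroker is a trigger actor that knocks out referenced lights when the BP_MementoMoriHero enters its box.
; The overlap calls Activate, which immediately plays audio on the LightAudio and HorrorLightAudio arrays.
; After a short delay, it sets intensity to zero on the Light and HorrorLight arrays, so sound leads the blackout.
; Nothing guards against retriggering, so each hero overlap runs it again.
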(event OnComponentBeginOverlap(Box)
  (params (OverlappedComponent :type Primitive%20Component%20Object%20Reference) (OtherActor :type Actor%20Object%20Reference) (OtherComp :type Primitive%20Component%20Object%20Reference) (OtherBodyIndex :type Integer) (bFromSweep :type Boolean) (SweepResult :type Hit%20Result%20Structure%20%28by%20ref%29))
  (Utilities|Casting|CastToBP_MementoMoriHero OtherActor)
  (CallFunction|Activate))

(event Custom|Activate
  (Utilities|FlowControl|Sequence
    (:then_0
      (Utilities|FlowControl|Delay 0.3)
      (for _array_element (Variables|Default|GetLight)
        (Rendering|Components|Light|SetIntensity (Variables|/Script/Engine.Light|GetLightComponent _array_element) 0.0))
      (for _array_element_2 (Variables|Default|GetHorrorLight)
        (Rendering|Components|Light|SetIntensity (Variables|/Game/Variant_Horror/Blueprints/Light/BP_HorrorLight.BP_HorrorLight_C|GetSpotLight _array_element_2) 0.0)))
    (:then_1
      (for _array_element_3 (Variables|Default|GetLightAudio)
        (Audio|Components|Audio|Play (Variables|/Game/MementoMori/Blueprints/Actors/BP_Audio.BP_Audio_C|GetAudio _array_element_3) 0.0))
      (for _array_element_4 (Variables|Default|GetHorrorLightAudio)
        (Audio|Components|Audio|Play (Variables|/Game/MementoMori/Blueprints/Actors/BP_Audio.BP_Audio_C|GetAudio _array_element_4) 0.0)))))

(fn ConstructionScript)