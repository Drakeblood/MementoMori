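; BP_DoorStampTrigger is a trigger actor that quickly shuts its referenced doors with a sound once the player is in position and looking the right way.
; When triggered, it re-checks on a short Delay loop until IsLookingGoodDirection passes and the player pawn overlaps its Box.
; It then shortens the doors' open time, closes them and plays the audio.
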(event EventTriggerEvent
  (if (and (CallFunction|IsLookingGoodDirection) (Collision|IsOverlappingActor (Variables|Default|GetBox) (Game|Player|GetPlayerPawn 0) :!class /Script/Engine.PrimitiveComponent)) :!label _label
    (Default|SetOpenTime (Variables|Default|GetDoors) 0.2)
    (Default|CloseDoor (Variables|Default|GetDoors))
    (Audio|Components|Audio|Play (Variables|/Game/MementoMori/Blueprints/Actors/BP_Audio.BP_Audio_C|GetAudio (Variables|Default|GetAudio)) 0.0)
    (else
      (Utilities|FlowControl|Delay 0.2)
      (goto _label))))

(fn ConstructionScript
  (|CallParentFunction))