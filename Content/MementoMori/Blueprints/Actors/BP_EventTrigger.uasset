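; BP_EventTrigger is a trigger volume actor that fires an event when the BP_MementoMoriHero character begins overlapping its box.
; TriggerEvent is empty here, serving as a hook for whatever the trigger should do.
; IsLookingGoodDirection is a helper that checks whether the player's view yaw, relative to the Arrow component, lies between MinRange and MaxRange.
; The overlap does not call this check.
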(event OnComponentBeginOverlap(Box)
  (params (OverlappedComponent :type Primitive%20Component%20Object%20Reference) (OtherActor :type Actor%20Object%20Reference) (OtherComp :type Primitive%20Component%20Object%20Reference) (OtherBodyIndex :type Integer) (bFromSweep :type Boolean) (SweepResult :type Hit%20Result%20Structure%20%28by%20ref%29))
  (if (.bSuccess (Utilities|Casting|CastToBP_MementoMoriHero OtherActor))
    (CallFunction|TriggerEvent)))

(event Custom|TriggerEvent)

(fn ConstructionScript)

(fn IsLookingGoodDirection
  (bind _returnvalue (Game|Player|GetPlayerPawn 0))
  (bind _arrow (Variables|Default|GetArrow))
  (bind _returnvalue_2 (Transformation|GetWorldRotation _arrow))
  (bind _outrotation (Actor|GetActorEyesViewPoint _returnvalue))
  (bind _returnvalue_3 (Math|Rotator|Delta(Rotator) _returnvalue_2 _outrotation))
  (return (and (> (.yaw _returnvalue_3) (Variables|Default|GetMinRange)) (< (.yaw _returnvalue_3) (Variables|Default|GetMaxRange)))))