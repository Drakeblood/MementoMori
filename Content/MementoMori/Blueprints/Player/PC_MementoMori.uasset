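; PC_MementoMori is the game's player controller, which sets up input and the HUD for the local player.
; On BeginPlay, it adds the default, horror and mouse-look Enhanced Input mapping contexts, then creates the WBP_HeroHUD widget and adds it to the viewport.
; The IA_Controls input action tells that HUD to show the controls.
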(event Input|EnhancedActionEvents|EnhancedInputActionIA_Controls
  (params (ActionValue :type Boolean) (ElapsedSeconds :type Float%20%28double-precision%29) (TriggeredSeconds :type Float%20%28double-precision%29) (InputAction :type Input%20Action%20Object%20Reference :default "/Game/Variant_Horror/Input/IA_Controls.IA_Controls"))
  (:Started
    (Default|ShowControls (Variables|Default|GetHeroHUD))))

(event EventBeginPlay
  (bind _returnvalue (PlayerController|LocalPlayerSubsystems|GetEnhancedInputLocalPlayerSubsystem))
  (if (Pawn|IsLocalPlayerController)
    (Utilities|FlowControl|Sequence
      (:then_0
        (Input|AddMappingContext _returnvalue "/Game/Input/IMC_Default.IMC_Default" 0 "(bIgnoreAllPressedKeysUntilRelease=True,bForceImmediately=False,bNotifyUserSettings=False)")
        (Input|AddMappingContext _returnvalue "/Game/Variant_Horror/Input/IMC_Horror.IMC_Horror" 0 "(bIgnoreAllPressedKeysUntilRelease=True,bForceImmediately=False,bNotifyUserSettings=False)")
        (Input|AddMappingContext _returnvalue "/Game/Input/IMC_MouseLook.IMC_MouseLook" 0 "(bIgnoreAllPressedKeysUntilRelease=True,bForceImmediately=False,bNotifyUserSettings=False)"))
      (:then_1
        (bind _returnvalue_2 (UserInterface|CreateWidget "/Game/MementoMori/Blueprints/UI/WBP_HeroHUD.WBP_HeroHUD_C"))
        (bind _output_get (Variables|Default|SetHeroHUD _returnvalue_2))
        (UserInterface|Viewport|AddtoViewport _output_get 0)))))

(fn ConstructionScript)