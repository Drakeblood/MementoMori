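; Baphomet character that leaves a ground trail and performs a jumpscare on the player.
; A looping timer traces downward while it moves fast enough and attaches timed decals at the hit point.
; WalkToRun plays a montage, then sets the Run flag.
; Jumpscare1 disables player input and both collisions, snaps Baphomet to face the player, plays montages and binds the hero's spring arm to an animated camera bone.
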(event Custom|TrailTick
  (bind _returnvalue (Transformation|GetActorUpVector))
  (bind _returnvalue_2 (Transformation|GetActorLocation))
  (bind _returnvalue_3 (* _returnvalue 5e+01))
  (bind _returnvalue_4 (+ _returnvalue_2 _returnvalue_3))
  (if (Variables|Default|GetShouldSpawnTrail)
    (if (> (Math|Vector|VectorLength (Transformation|GetVelocity)) (Variables|Default|GetTrailMinSpeed))
      (bind _outhit (Collision|LineTraceByChannel _returnvalue_4 (- _returnvalue_4 (* _returnvalue 2e+03)) "TraceTypeQuery1" false 0 "None"))
      (if (.bblockinghit _outhit)
        (Class|GameplayStatics|SpawnDecalAttached (Variables|Default|GetTrailMaterial) (Variables|Default|GetTrailSize) (.hitcomponent _outhit) "None" (+ (.impactpoint _outhit) (* (.impactnormal _outhit) 2.0)) "0, 0, 0" "KeepWorldPosition" (Variables|Default|GetTrailLifeSpan))))))

(event Custom|WalkToRun
  (Animation|Montage|PlayMontage (Variables|Character|GetMesh) "/Game/MementoMori/Character/AM_Bathomet.AM_Bathomet"
    (:OnCompleted
      _)
    (:OnBlendOut
      _)
    (:OnInterrupted
      _))
  (Variables|Default|SetRun true))

(event Custom|Jumpscare1
  (params (MontageToPlay :type Anim%20Montage%20Object%20Reference))
  (bind _returnvalue (Game|Player|GetPlayerPawn 0))
  (Collision|SetActorEnableCollision (Game|Player|GetPlayerPawn 0) false)
  (Collision|SetActorEnableCollision false)
  (Input|DisableInput _returnvalue (Game|GetPlayerController 0))
  (Transformation|SetActorLocationAndRotation (.location (Transformation|GetActorTransform _returnvalue)) (Math|Conversions|RotationFromXVector (* (Transformation|GetActorForwardVector (Game|Player|GetPlayerPawn 0)) -1.0)))
  (Animation|Montage|PlayMontage (Variables|Character|GetMesh) MontageToPlay
    (:then
      (Transformation|AddActorWorldOffset (+ (* (Transformation|GetActorForwardVector) -5e+01) "0.000000,0.000000,-33.284000" "0.000000,0.000000,-33.284000" "0.000000,0.000000,-33.284000" "0.000000,0.000000,-12.000000"))
      (bind _asbp_memento_mori_hero (Utilities|Casting|CastToBP_MementoMoriHero (Game|Player|GetPlayerPawn 0)))
      (Variables|/Script/Engine.SpringArmComponent|SetbUsePawnControlRotation (Variables|/Game/MementoMori/Blueprints/Character/BP_MementoMoriHero.BP_MementoMoriHero_C|GetSpringArm _asbp_memento_mori_hero) false)
      (Transformation|AttachComponentToComponent (Variables|/Game/MementoMori/Blueprints/Character/BP_MementoMoriHero.BP_MementoMoriHero_C|GetSpringArm _asbp_memento_mori_hero) (Variables|/Game/MementoMori/Blueprints/Character/BP_MementoMoriHero.BP_MementoMoriHero_C|GetFirstPersonMesh _asbp_memento_mori_hero) "Camera_Bone" "SnapToTarget" "SnapToTarget" "KeepWorld" true)
      (Transformation|AttachComponentToComponent (Variables|/Game/MementoMori/Blueprints/Character/BP_MementoMoriHero.BP_MementoMoriHero_C|GetFirstPersonMesh _asbp_memento_mori_hero) (Variables|/Script/Engine.Character|GetCapsuleComponent _asbp_memento_mori_hero) "None" "KeepWorld" "KeepWorld" "KeepWorld" true)
      (Components|Animation|PlayAnimation (Variables|/Game/MementoMori/Blueprints/Character/BP_MementoMoriHero.BP_MementoMoriHero_C|GetFirstPersonMesh _asbp_memento_mori_hero) "/Game/MementoMori/Character/Player/PlayerJumpscare3_Anim_Player_Jumpscare1.PlayerJumpscare3_Anim_Player_Jumpscare1" false))))

(event EventBeginPlay
  (|CallParentFunction)
  (Utilities|Time|SetTimerbyEvent (delegate Custom|TrailTick) (Variables|Default|GetTrailInterval) true))

(event Collision|EventActorBeginOverlap
  (params (OtherActor :type Actor%20Object%20Reference))
  (|CallParentFunction OtherActor) ; This node is disabled and will not be called.\nDrag off pins to build functionality.
)

(event EventTick
  (params (DeltaSeconds :type Float%20%28single-precision%29))
  (|CallParentFunction DeltaSeconds))

(fn ConstructionScript
  (|CallParentFunction))