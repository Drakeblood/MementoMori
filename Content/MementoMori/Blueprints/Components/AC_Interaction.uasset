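; Actor component on the MementoMori hero that handles first-hand detection and use of objects implementing BPI_Interactable.
; Each tick, unless an interaction is ongoing, a camera-forward line trace picks the target, checks it can be interacted with, toggles its focus and shows or hides the HUD prompt.
; TryInteract begins the interaction and remembers ongoing ones, so the next call ends that interaction instead.
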(event Custom|TryInteract
  (bind _currentongoinginteractable (Variables|Default|GetCurrentOngoingInteractable)
    (:then
      (Class|BPIInteractable|EndInteract(Message) _currentongoinginteractable (Variables|Default|GetHero))
      (Variables|Default|SetCurrentOngoingInteractable 0))
    (:else
      (bind _currentinteractable (Variables|Default|GetCurrentInteractable)
        (:then
          (Class|BPIInteractable|BeginInteract(Message) _currentinteractable (Variables|Default|GetHero))
          (bind _ongoing (Class|BPIInteractable|IsOngoingInteraction(Message) _currentinteractable))
          (Development|PrintString (Utilities|String|Append "Interacted with: " (Utilities|GetDisplayName _currentinteractable) " is Ongoing: " (Utilities|String|ToString(Boolean) _ongoing)) false)
          (if _ongoing
            (Variables|Default|SetCurrentOngoingInteractable (Variables|Default|GetCurrentInteractable)))
          (Class|BPIInteractable|DeFocus(Message) (Variables|Default|GetCurrentInteractable) (Variables|Default|GetHero))
          (Variables|Default|SetCurrentInteractable 0)
          (Default|HideInteractionMessage (Variables|/Game/MementoMori/Blueprints/Player/PC_MementoMori.PC_MementoMori_C|GetHeroHUD (.AsPC%20Memento%20Mori (Utilities|Casting|CastToPC_MementoMori (Game|GetPlayerController 0))))))
        (:else)))))

(event EventBeginPlay
  (Variables|Default|SetHero (.AsBP%20Memento%20Mori%20Hero (Utilities|Casting|CastToBP_MementoMoriHero (Components|GetOwner)))))

(event EventTick
  (params (DeltaSeconds :type Float%20%28single-precision%29))
  (bind _hero (Variables|Default|GetHero))
  (bind _camera (Variables|/Game/MementoMori/Blueprints/Character/BP_MementoMoriHero.BP_MementoMoriHero_C|GetCamera _hero))
  (bind _returnvalue (Transformation|GetWorldLocation _camera))
  (Variables|Default|GetCurrentOngoingInteractable
    (:then)
    (:else
      (bind (_outhit _returnvalue_2) (Collision|LineTraceByChannel _returnvalue (+ _returnvalue (* (Math|Vector|GetForwardVector _camera) (Variables|Default|GetLineTraceLength))) "TraceTypeQuery3" false 0 "None" true "(R=1.000000,G=0.000000,B=0.000000,A=1.000000)" "(R=0.000000,G=1.000000,B=0.000000,A=1.000000)" 0.1))
      (if (and (Utilities|DoesObjectImplementInterface (.hitactor _outhit) "/Game/MementoMori/Blueprints/Interfaces/BPI_Interactable.BPI_Interactable_C") _returnvalue_2)
        (if (!= (Variables|Default|GetCurrentInteractable) (.hitactor _outhit))
          (bind _newparam (Class|BPIInteractable|CanInteract(Message) (.hitactor _outhit) (Variables|Default|GetHero)))
          (if _newparam
            (bind _currentinteractable (Variables|Default|GetCurrentInteractable)
              (:then
                (Class|BPIInteractable|DeFocus(Message) _currentinteractable (Variables|Default|GetHero)))
              (:else
                _))
            (bind _output_get (Variables|Default|SetCurrentInteractable (.hitactor _outhit)))
            (Class|BPIInteractable|Focus(Message) _output_get (Variables|Default|GetHero))
            (bind _message (Class|BPIInteractable|GetInteractionMessage(Message) (Variables|Default|GetCurrentInteractable) (Variables|Default|GetHero)))
            (Default|ShowInteractionMessage (Variables|/Game/MementoMori/Blueprints/Player/PC_MementoMori.PC_MementoMori_C|GetHeroHUD (.AsPC%20Memento%20Mori (Utilities|Casting|CastToPC_MementoMori (Game|GetPlayerController 0)))) _message)
            (else
              (bind _currentinteractable_2 (Variables|Default|GetCurrentInteractable :!label _label)
                (:then
                  (Class|BPIInteractable|DeFocus(Message) _currentinteractable_2 (Variables|Default|GetHero))
                  (Variables|Default|SetCurrentInteractable 0)
                  (Default|HideInteractionMessage (Variables|/Game/MementoMori/Blueprints/Player/PC_MementoMori.PC_MementoMori_C|GetHeroHUD (.AsPC%20Memento%20Mori (Utilities|Casting|CastToPC_MementoMori (Game|GetPlayerController 0))))))
                (:else)))))
        (else
          (goto _label))))))