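; AC_PickUp is an actor component that lets the BP_MementoMoriHero pick up, carry and release physical items.
; On BeginPlay it caches the hero and its PhysicsHandle, which PickUpItem uses to grab a component at a given location and rotation.
; While something is held, Tick moves the handle's target to the hero's PickUpHandleScene location, updating position only, until ReleaseItem drops it.
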(event Custom|PickUpItem
  (params (Component :type Primitive%20Component%20Object%20Reference) (InBoneName :type Name) (Location :type Vector) (Rotation :type Rotator))
  (Physics|Components|PhysicsHandle|GrabComponentatLocationwithRotation (Variables|Default|GetPhysicsHandle) Component InBoneName Location Rotation))

(event Custom|ReleaseItem
  (Physics|Components|PhysicsHandle|ReleaseComponent (Variables|Default|GetPhysicsHandle)))

(event EventBeginPlay
  (bind _output_get (Variables|Default|SetHero (.AsBP%20Memento%20Mori%20Hero (Utilities|Casting|CastToBP_MementoMoriHero (Components|GetOwner)))))
  (Variables|Default|SetPhysicsHandle (Variables|/Game/MementoMori/Blueprints/Character/BP_MementoMoriHero.BP_MementoMoriHero_C|GetPhysicsHandle _output_get)))

(event EventTick
  (params (DeltaSeconds :type Float%20%28single-precision%29))
  (if (!= (Class|PhysicsHandleComponent|GetGrabbedComponent (Variables|Default|GetPhysicsHandle)) 0)
    (Physics|Components|PhysicsHandle|SetTargetLocation (Variables|Default|GetPhysicsHandle) (Transformation|GetWorldLocation (Variables|/Game/MementoMori/Blueprints/Character/BP_MementoMoriHero.BP_MementoMoriHero_C|GetPickUpHandleScene (Variables|Default|GetHero))))))